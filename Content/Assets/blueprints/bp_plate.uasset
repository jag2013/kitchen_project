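; Plate actor for a dishwashing game that can be washed for points, clank, or shatter.
; WashEvent swaps to the clean plate material after a delay, then destroys the actor and adds to the player pawn's score.
; BreakDish reports a broken dish, replaces the static mesh with a destructible mesh fractured by radius damage, then turns off collision and removes the debris after delays.
; ClankEvent plays an attenuated clank sound at the plate.
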(event Custom|ClankEvent
  (Audio|PlaySoundatLocation "/Game/Assets/audio/dish_clank_01_Cue.dish_clank_01_Cue" (Transformation|GetWorldLocation (Variables|Default|GetStaticMesh)) "0, 0, 0" 0.8 1.0 0.0 "/Game/Assets/attenuation/DishClankAttenuation.DishClankAttenuation"))

(event Custom|WashEvent
  (Utilities|FlowControl|Delay 5.0)
  (Rendering|Material|SetMaterial (Variables|Default|GetStaticMesh) 0 "/Game/Assets/material/m_plate.m_plate")
  (Utilities|FlowControl|Delay 5.0)
  (Actor|DestroyActor)
  (Class|BPIPlayer|AddtoScore(Message) (Game|Player|GetPlayerPawn 0) 1))

(event Custom|BreakDish
  (bind _destructible (Variables|Default|GetDestructible))
  (Class|BPIPlayer|AddtoBrokenDishScore(Message) (Game|Player|GetPlayerPawn 0) 1)
  (Rendering|SetVisibility (Variables|Default|GetStaticMesh) false false)
  (Collision|SetCollisionResponsetoAllChannels (Variables|Default|GetStaticMesh) "ECR_Ignore")
  (Components|DestroyComponent (Variables|Default|GetStaticMesh))
  (Audio|PlaySoundatLocation "/Game/Assets/audio/plate_break_cue.plate_break_cue" (Transformation|GetWorldLocation (Variables|Default|GetDestructible)) "0, 0, 0" 1.0 1.0 0.0 "/Game/Assets/attenuation/PlateBreakAttenuation.PlateBreakAttenuation")
  (Class|DestructibleComponent|SetDestructibleMesh _destructible "/Game/Assets/meshes/plate_DM.plate_DM")
  (Class|DestructibleComponent|ApplyRadiusDamage _destructible 5.0 (Transformation|GetWorldLocation _destructible) 5.0 0.0 true)
  (Utilities|FlowControl|Delay 1.0)
  (Collision|SetCollisionResponsetoAllChannels (Variables|Default|GetDestructible) "ECR_Ignore")
  (Collision|SetCollisionResponsetoAllChannels (Variables|Default|GetPlateCollision_Floor) "ECR_Ignore")
  (Utilities|FlowControl|Delay 6.0)
  (Rendering|SetVisibility (Variables|Default|GetDestructible) false false)
  (Actor|DestroyActor))

(fn ConstructionScript)