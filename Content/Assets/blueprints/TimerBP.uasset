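; TimerBP is a timer actor that plays an alarm sound at its Widget component's world location.
; On BeginPlay it takes the first MyVRGamemode actor and binds a custom event to its alarm dispatcher, which plays the timer alarm cue when fired.
; A separate Alarm function plays the same cue with attenuation settings, while the TimerAlarm event is empty.
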(event Custom|AlarmDispatchCustomEvent
  (Audio|PlaySoundatLocation "/Game/Assets/audio/timer_alarm_cue.timer_alarm_cue" (Transformation|GetWorldLocation (Variables|Default|GetWidget))))

(event EventBeginPlay
  (bind _outactors (Actor|GetAllActorsOfClass "/Game/Assets/player/MyVRGameMode.MyVRGamemode_C"))
  (bind _output_get (Variables|Default|SetVRGameMode (Utilities|Array|Get(acopy) _outactors)))
  (EventDispatchers|BindEventtoAlarmDispatch _output_get (delegate Custom|AlarmDispatchCustomEvent)))

(event EventTimerAlarm)

(fn ConstructionScript)

(fn Alarm
  (Audio|PlaySoundatLocation "/Game/Assets/audio/timer_alarm_cue.timer_alarm_cue" (Transformation|GetWorldLocation (Variables|Default|GetWidget)) "0, 0, 0" 1.0 1.0 0.0 "/Game/Assets/attenuation/TimerAlarmAttenuation.TimerAlarmAttenuation"))